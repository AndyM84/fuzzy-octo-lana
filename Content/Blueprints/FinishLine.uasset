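; Finish line actor that brings up the finish menu when the player passes through it.
; When an actor stops overlapping FinishLineVolume, it checks that the actor is player 0's pawn and that Game_HUD's ShowFinishMenu flag is off, then calls ToggleFinishMenu on that HUD.
; The trigger fires on exiting the volume, and the flag check keeps a repeat crossing from toggling a menu that is already showing.
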(event OnComponentEndOverlap(FinishLineVolume)
  (params (OtherActor :type Actor%20Object%20Reference) (OtherComp :type Primitive%20Component%20Object%20Reference) (OtherBodyIndex :type Integer))
  (bind _asgame_hud_c (Utilities|Casting|CastToGame_HUD (HUD|GetHUD (Game|GetPlayerController 0))))
  (if (not (Variables|/Game/HUD/Blueprints/Game_HUD.Game_HUD_C|GetShowFinishMenu _asgame_hud_c))
    (if (== OtherActor (Game|Player|GetPlayerPawn 0))
      (bind _asgame_hud_c_2 (Utilities|Casting|CastToGame_HUD (HUD|GetHUD (Game|GetPlayerController 0))))
      (Default|ToggleFinishMenu _asgame_hud_c_2))))

(fn ConstructionScript)